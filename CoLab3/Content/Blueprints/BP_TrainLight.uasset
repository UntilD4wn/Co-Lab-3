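; BP_TrainLight is a searchlight that detects the player, with Train and Watchtower variants driven by looping Level Sequences.
; A looping timer sphere-traces for pawns along the spotlight, then line-traces to the player so "Wall"-tagged actors block detection.
; On detection, Train flashes red and calls the player's LightKill, while Watchtower pauses its sweep, turns red and alerts BP_AI.
; Train move and sweep-transition logic is disconnected, and RotateSpotlight is empty.
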(event Custom|PauseWatchtower
  ;[0.1298 0.4691 0.7552 0.5] SearchLight stationary sweep
  (Sequencer|Player|Pause (Variables|/Script/LevelSequence.LevelSequenceActor|GetSequencePlayer (Variables|Default|GetWatchtowerSweep%20ref))))

(event Custom|PlayerSpotted
  ;[0.1298 0.4691 0.7552 0.5] Player Detected - (Train level Searchlight)
  (bind _outactor (Sequencer|Player|CreateLevelSequencePlayer "/Game/Blueprints/Sequences/S_LightsRed.S_LightsRed"))
  (Sequencer|Player|Play (Variables|/Script/LevelSequence.LevelSequenceActor|GetSequencePlayer _outactor) :!class /Script/MovieScene.MovieSceneSequencePlayer)
  (bind _outactor_2 (Sequencer|Player|CreateLevelSequencePlayer "/Game/Blueprints/Sequences/S_LightStripRed.S_LightStripRed"))
  (Sequencer|Player|Play (Variables|/Script/LevelSequence.LevelSequenceActor|GetSequencePlayer _outactor_2) :!class /Script/MovieScene.MovieSceneSequencePlayer))

(event Custom|REdspotlight
  (Rendering|Components|Light|SetLightColor (Variables|Default|GetSpotLight) "(R=1.000000,G=0.000000,B=0.000000,A=1.000000)" true)
  (Utilities|FlowControl|Delay 2.0)
  (Rendering|Components|Light|SetLightColor (Variables|Default|GetSpotLight) "(R=0.637153,G=0.637153,B=0.637153,A=1.000000)" true))

(event Custom|PauseSweep
  (bind _searchlightsweep_ref (Variables|Default|GetSearchLightSweep%20Ref))
  (bind _sequenceplayer (Variables|/Script/LevelSequence.LevelSequenceActor|GetSequencePlayer _searchlightsweep_ref))
  ;[0.1298 0.4691 0.7552 0.5] Pause Sweep
  (Sequencer|Player|Pause _sequenceplayer)
  (Utilities|FlowControl|Delay 0.4)
  (Sequencer|Player|Play _sequenceplayer :!class /Script/MovieScene.MovieSceneSequencePlayer))

(event Custom|RotateSpotlight
  ;[0.1298 0.4691 0.7552 0.5] SearchLight stationary sweep
)

(event Custom|S
  ;[1 0.3329 0.1823 0.5] Start Sequences depending on which type of Searchlight
  (bind _outactor (Sequencer|Player|CreateLevelSequencePlayer "/Game/Blueprints/Sequences/S_TrainRight.S_TrainRight"))
  (bind _output_get (Variables|Default|SetTrainSequence%20Ref _outactor))
  (Class|MovieSceneSequencePlayer|PlayLooping (Variables|/Script/LevelSequence.LevelSequenceActor|GetSequencePlayer _output_get) -1))

(event Custom|delay
  (Utilities|FlowControl|Delay 1.0))

(event EventBeginPlay
  (Utilities|FlowControl|Sequence
    (:then_0
      ;[0.4183 0.14 0.9271 0.5] Start Traces
      (Variables|Default|SetHasBeenDetected false)
      (bind _returnvalue (Actor|GetActorOfClass "/Game/Blueprints/BP_Train.BP_Train_C"))
      (bind _returnvalue_2 (Actor|GetActorOfClass "/Game/Blueprints/waypointAIPath/BP_AI.BP_AI_C"))
      (Variables|Default|SetActors%20to%20Ignore (Utilities|Array|MakeArray _returnvalue_2 _returnvalue))
      (Utilities|Time|SetTimerbyFunctionName 0 "TraceEnemies" 0.2 true))
    (:then_1
      ;[1 0.3329 0.1823 0.5] Start Sequences depending on which type of Searchlight
      (switch Utilities|FlowControl|Switch|SwitchonE_SearchLightVersion (Variables|Default|GetSearchLight%20Version)
        (:NewEnumerator1
          (CallFunction|RotateSpotlight))
        (:NewEnumerator2
          (Utilities|FlowControl|Delay 1.5)
          (CallFunction|S))
        (:NewEnumerator3
          ;[0.1298 0.4691 0.7552 0.5] SearchLight stationary sweep
          (bind _outactor (Sequencer|Player|CreateLevelSequencePlayer "/Game/Blueprints/Sequences/S_Sweep.S_Sweep"))
          (bind _output_get (Variables|Default|SetWatchtowerSweep%20ref _outactor))
          (Class|MovieSceneSequencePlayer|PlayLooping (Variables|/Script/LevelSequence.LevelSequenceActor|GetSequencePlayer _output_get) -1))))
    (:then_2
      (bind _returnvalue_3 (Actor|GetActorOfClass "/Game/Blueprints/waypointAIPath/BP_AI.BP_AI_C"))
      (Variables|Default|SetEnemy%20Ref _returnvalue_3))))

(fn ConstructionScript)

(fn TraceEnemies
  (bind _spotlight (Variables|Default|GetSpotLight))
  (bind _returnvalue (Transformation|GetWorldLocation _spotlight))
  (if (not (Variables|Default|GetIsPlayerDetected))
    ;[1 0.5164 0.25 0.5] Generates Multi Sphere trace
    (bind _outhits (Collision|MultiSphereTraceForObjects _returnvalue (+ _returnvalue (* (Math|Vector|GetForwardVector _spotlight) (Variables|/Script/Engine.LocalLightComponent|GetAttenuationRadius _spotlight))) (Variables|Default|GetDetectionRadius) (Utilities|Array|MakeArray "ObjectTypeQuery3") false (Variables|Default|GetActors%20to%20Ignore) "None"))
    (Variables|Default|SetIsPlayerDetected false)
    ;[1 0.3854 0.579 0.5] Checks if hit result (player) was valid - sends a line trace to player location
    (for _array_element _outhits
      (Variables|Default|SetArray%20Element "")
      (Utilities|IsValid (.HitActor (Collision|BreakHitResult _array_element))
        (:Is%20Valid
          (bind _returnvalue_2 (Actor|GetActorOfClass "/Game/ThirdPerson/Blueprints/BP_ThirdPersonCharacter.BP_ThirdPersonCharacter_C"))
          (Variables|Default|SetPlayer%20Location (Transformation|GetActorLocation _returnvalue_2))
          (bind _outhit (Collision|LineTraceByChannel (Transformation|GetWorldLocation (Variables|Default|GetSpotLight)) (Transformation|GetActorLocation _returnvalue_2) "TraceTypeQuery1" false (Variables|Default|GetActors%20to%20Ignore) "None"))
          ;[0.6706 0.3438 1 0.5] Checks if theres a blocking wall detected in front of the player - if not the player is detected
          (bind _output_get (Variables|Default|SetIsPlayerDetected (not (Actor|ActorHasTag (.HitActor (Collision|BreakHitResult _outhit)) "Wall"))))
          (if _output_get
            (Variables|Default|SetIsPlayerDetected false)
            (switch Utilities|FlowControl|Switch|SwitchonE_SearchLightVersion (Variables|Default|GetSearchLight%20Version)
              (:NewEnumerator1
                (CallFunction|PauseSweep))
              (:NewEnumerator2
                (bind _returnvalue_3 (Actor|GetActorOfClass "/Game/Blueprints/BP_Train.BP_Train_C"))
                (Default|Red _returnvalue_3)
                (CallFunction|REdspotlight)
                (bind _returnvalue_4 (Actor|GetActorOfClass "/Game/ThirdPerson/Blueprints/BP_ThirdPersonCharacter.BP_ThirdPersonCharacter_C"))
                (Default|LightKill _returnvalue_4)
                (Default|Red _returnvalue_3))
              (:NewEnumerator3
                (CallFunction|PauseWatchtower)
                (Rendering|Components|Light|SetLightColor (Variables|Default|GetSpotLight) "(R=0.869792,G=0.000000,B=0.000000,A=1.000000)" true)
                (bind _returnvalue_5 (Actor|GetActorOfClass "/Game/Blueprints/waypointAIPath/BP_AI.BP_AI_C"))
                (Default|LightSpottedPlayer _returnvalue_5)))
            (else
              (return))))))))