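; BP_Train is a train actor whose Red event toggles the train lighting to and from red.
; The event creates new players for the light and light-strip level sequences, playing them forward or in reverse according to a LightsChanged flag.
; The flag becomes true after a short delay on the forward pass and clears immediately on reverse.
; Direct spotlight recoloring nodes remain but never run.
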(event Custom|Red
  (if (not (Variables|Default|GetLightsChanged))
    (bind _outactor (Sequencer|Player|CreateLevelSequencePlayer "/Game/Blueprints/Sequences/S_LightsRed.S_LightsRed"))
    (Sequencer|Player|Play (Variables|/Script/LevelSequence.LevelSequenceActor|GetSequencePlayer _outactor) :!class /Script/MovieScene.MovieSceneSequencePlayer)
    (bind _outactor_2 (Sequencer|Player|CreateLevelSequencePlayer "/Game/Blueprints/Sequences/S_LightStripRed.S_LightStripRed"))
    (Sequencer|Player|Play (Variables|/Script/LevelSequence.LevelSequenceActor|GetSequencePlayer _outactor_2) :!class /Script/MovieScene.MovieSceneSequencePlayer)
    (Utilities|FlowControl|Delay 1.0)
    (Variables|Default|SetLightsChanged true)
    (else
      (bind _outactor_3 (Sequencer|Player|CreateLevelSequencePlayer "/Game/Blueprints/Sequences/S_LightsRed.S_LightsRed"))
      (Class|MovieSceneSequencePlayer|PlayReverse (Variables|/Script/LevelSequence.LevelSequenceActor|GetSequencePlayer _outactor_3))
      (bind _outactor_4 (Sequencer|Player|CreateLevelSequencePlayer "/Game/Blueprints/Sequences/S_LightStripRed.S_LightStripRed"))
      (Class|MovieSceneSequencePlayer|PlayReverse (Variables|/Script/LevelSequence.LevelSequenceActor|GetSequencePlayer _outactor_4))
      (Variables|Default|SetLightsChanged false))))

(event EventBeginPlay)

(event Collision|EventActorBeginOverlap
  (params (OtherActor :type Actor%20Object%20Reference)))

(event EventTick
  (params (DeltaSeconds :type Float%20%28single-precision%29)))

(fn ConstructionScript)