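; BP_AI is an AI pawn that patrols an array of waypoints in a loop and moves toward pawns it sees.
; FollowWaypoint uses AI MoveTo, advancing the wrapping index on success and calling itself again after a short pause.
; PawnSensing redirects movement to the seen pawn, with a brief retriggerable delay that resumes patrol once sightings stop refreshing it.
; EnemyAppear, lightspottedplayer and Reset are empty, and some tag-check and teleport logic is disconnected.
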(event OnSeePawn(PawnSensing)
  (params (Pawn :type Pawn%20Object%20Reference))
  (AI|AIMoveTo self "0, 0, 0" Pawn 5.0 false
    (:then
      (Utilities|FlowControl|RetriggerableDelay 0.1)
      (CallFunction|FollowWaypoint))))

(event Custom|FollowWaypoint
  (AI|AIMoveTo self "0, 0, 0" (Utilities|Array|Get(acopy) (Variables|Default|Getwaypoints) (Variables|Default|Getcurrentwaypoint)) 5.0 false
    (:OnSuccess
      (Math|Integer|IncrementInt (Variables|Default|Getcurrentwaypoint)
        (:%20%20
          (if (>= (Variables|Default|Getcurrentwaypoint) (Utilities|Array|Length (Variables|Default|Getwaypoints)))
            (Variables|Default|Setcurrentwaypoint 0))
          (Utilities|FlowControl|Delay 0.5)
          (CallFunction|FollowWaypoint))))))

(event Custom|EnemyAppear)

(event Custom|light%20spotted%20player)

(event Custom|Reset)

(event EventBeginPlay
  (CallFunction|FollowWaypoint))

(fn ConstructionScript)