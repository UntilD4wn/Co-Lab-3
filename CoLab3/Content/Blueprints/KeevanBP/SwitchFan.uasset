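; SwitchFan is a switchable fan that floats characters upward while they are inside its capsule volume.
; A SwitchOn/Off event toggles the IsFanOn flag, which is checked only when an overlap begins.
; On entry while on, it inverts the character's gravity scale, sets an upward velocity and adds a downward force.
; Leaving the capsule restores normal gravity scale regardless of the fan's state.
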(event OnComponentBeginOverlap(Capsule)
  (params (OverlappedComponent :type Primitive%20Component%20Object%20Reference) (OtherActor :type Actor%20Object%20Reference) (OtherComp :type Primitive%20Component%20Object%20Reference) (OtherBodyIndex :type Integer) (bFromSweep :type Boolean) (SweepResult :type Hit%20Result%20Structure%20%28by%20ref%29))
  (if (Variables|Default|GetIsFanOn?)
    (bind _ascharacter (Utilities|Casting|CastToCharacter OtherActor)
      (:then
        (Variables|/Script/Engine.CharacterMovementComponent|SetGravityScale (Variables|/Script/Engine.Character|GetCharacterMovement _ascharacter) -1.0)
        (Variables|/Script/Engine.MovementComponent|SetVelocity (Variables|/Script/Engine.Character|GetCharacterMovement _ascharacter) (Math|Vector|MakeVector 0.0 0.0 1e+02))
        (Physics|AddForce (Variables|/Script/Engine.Character|GetCharacterMovement _ascharacter) "0.000000,0.000000,-100.000000"))
      (:CastFailed
        (Development|PrintString "Error")))))

(event OnComponentEndOverlap(Capsule)
  (params (OverlappedComponent :type Primitive%20Component%20Object%20Reference) (OtherActor :type Actor%20Object%20Reference) (OtherComp :type Primitive%20Component%20Object%20Reference) (OtherBodyIndex :type Integer))
  (bind _ascharacter (Utilities|Casting|CastToCharacter OtherActor))
  (Variables|/Script/Engine.CharacterMovementComponent|SetGravityScale (Variables|/Script/Engine.Character|GetCharacterMovement _ascharacter) 1.0))

(event Custom|SwitchOn/Off
  (if (Variables|Default|GetIsFanOn?)
    (Variables|Default|SetIsFanOn? false)
    (else
      (Variables|Default|SetIsFanOn? true))))

(fn ConstructionScript)