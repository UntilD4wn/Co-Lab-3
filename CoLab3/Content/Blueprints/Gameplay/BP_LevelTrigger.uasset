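; Level transition trigger that loads another map when any actor begins overlapping it.
; A LevelNumber variable selects the destination by hard-coded name through a switch, covering the subway, warehouse and lab levels plus the main menu.
; The overlapping actor is not filtered, and a leftover tag-check chain in the event graph never runs.
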(event Collision|EventActorBeginOverlap
  (params (OtherActor :type Actor%20Object%20Reference))
  (switch int (Variables|Default|GetLevelNumber)
    (:1
      (Game|OpenLevel(byName) "Subway_assetsadded"))
    (:2
      (Game|OpenLevel(byName) "Warehouse1"))
    (:3
      (Game|OpenLevel(byName) "LabPart1"))
    (:4
      (Game|OpenLevel(byName) "Lab_Platforms"))
    (:5
      (Game|OpenLevel(byName) "Lab"))
    (:6
      (Game|OpenLevel(byName) "MainMenu"))))

(fn ConstructionScript)