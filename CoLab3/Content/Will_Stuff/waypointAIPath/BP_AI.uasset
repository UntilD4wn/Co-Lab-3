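; BP_AI is an enemy pawn that patrols waypoints, chases pawns it sees and kills the player on contact.
; A looping AIMoveTo cycles through the Waypoints array, pausing briefly after each successful move.
; PawnSensing redirects movement to the seen pawn, with a retriggerable delay resuming patrol shortly after the last sighting.
; Any capsule overlap calls LightKill on the BP_ThirdPersonCharacter found by class, without checking the overlapping actor.
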(event OnComponentBeginOverlap(CapsuleComponent)
  (params (OverlappedComponent :type Primitive%20Component%20Object%20Reference) (OtherActor :type Actor%20Object%20Reference) (OtherComp :type Primitive%20Component%20Object%20Reference) (OtherBodyIndex :type Integer) (bFromSweep :type Boolean) (SweepResult :type Hit%20Result%20Structure%20%28by%20ref%29))
  (bind _returnvalue (Actor|GetActorOfClass "/Game/ThirdPerson/Blueprints/BP_ThirdPersonCharacter.BP_ThirdPersonCharacter_C"))
  (Default|LightKill _returnvalue))

(event OnSeePawn(PawnSensing)
  (params (Pawn :type Pawn%20Object%20Reference))
  (AI|AIMoveTo self "0, 0, 0" Pawn 5.0 false
    (:then
      (Utilities|FlowControl|RetriggerableDelay 2.0)
      (CallFunction|FollowWaypoint))))

(event Custom|FollowWaypoint
  (AI|AIMoveTo self "0, 0, 0" (Utilities|Array|Get(acopy) (Variables|Default|Getwaypoints) (Variables|Default|Getcurrentwaypoint)) 5.0 false
    (:OnSuccess
      (Math|Integer|IncrementInt (Variables|Default|Getcurrentwaypoint)
        (:%20%20
          (if (>= (Variables|Default|Getcurrentwaypoint) (Utilities|Array|Length (Variables|Default|Getwaypoints)))
            (Variables|Default|Setcurrentwaypoint 0))
          (Utilities|FlowControl|Delay 0.1)
          (CallFunction|FollowWaypoint))))))

(event EventBeginPlay
  (CallFunction|FollowWaypoint))

(fn ConstructionScript)