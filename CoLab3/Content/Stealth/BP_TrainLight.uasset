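; Stealth searchlight actor that plays a looping sweep sequence, or a one-shot train sequence for the Train version.
; A looping timer sphere-traces along the spotlight for pawns, then line-traces to the player character, ignoring the train.
; Unless that trace hits a "Wall"-tagged actor, it prints a debug message and briefly pauses the sweep.
; PlayerSpotted, which stops the sequence and moves the train toward the player's Y, is never called here.
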(event Custom|PlayerSpotted
  ;[0.1298 0.4691 0.7552 0.5] Player Detected - (Train level Searchlight)
  (Utilities|FlowControl|Delay 0.5)
  (Sequencer|Player|Stop (Variables|/Script/LevelSequence.LevelSequenceActor|GetSequencePlayer (Variables|Default|GetTrainSequence%20Ref)) :!class /Script/MovieScene.MovieSceneSequencePlayer)
  (Utilities|FlowControl|Delay 0.5)
  (bind _returnvalue (Actor|GetActorOfClass "/Game/Stealth/BP_Train.BP_Train_C"))
  (Components|MoveComponentTo (Variables|/Game/Stealth/BP_Train.BP_Train_C|GetDefaultSceneRoot _returnvalue) (Math|Vector|MakeVector -385.0 (.y (Variables|Default|GetPlayer%20Location)) 575.0) "0.000000,90.000000,0.000000" true true 2.0 false))

(event Custom|PauseSweep
  (bind _searchlightsweep_ref (Variables|Default|GetSearchLightSweep%20Ref))
  (bind _sequenceplayer (Variables|/Script/LevelSequence.LevelSequenceActor|GetSequencePlayer _searchlightsweep_ref))
  ;[0.1298 0.4691 0.7552 0.5] Pause Sweep
  (Sequencer|Player|Pause _sequenceplayer)
  (Utilities|FlowControl|Delay 0.4)
  (Sequencer|Player|Play _sequenceplayer :!class /Script/MovieScene.MovieSceneSequencePlayer))

(event Custom|RotateSpotlight
  ;[0.1298 0.4691 0.7552 0.5] SearchLight stationary sweep
  (bind _outactor (Sequencer|Player|CreateLevelSequencePlayer "/Game/Stealth/Sequences/S_TrainLight.S_TrainLight"))
  (bind _output_get (Variables|Default|SetSearchLightSweep%20Ref _outactor))
  (Class|MovieSceneSequencePlayer|PlayLooping (Variables|/Script/LevelSequence.LevelSequenceActor|GetSequencePlayer _output_get) 2))

(event EventBeginPlay
  (Utilities|FlowControl|Sequence
    (:then_0
      ;[0.4183 0.14 0.9271 0.5] Start Traces
      (Variables|Default|SetHasBeenDetected false)
      (bind _returnvalue (Actor|GetActorOfClass "/Game/Stealth/BP_Train.BP_Train_C"))
      (Variables|Default|SetActors%20to%20Ignore (Utilities|Array|MakeArray _returnvalue))
      (Utilities|Time|SetTimerbyFunctionName 0 "TraceEnemies" 0.2 true))
    (:then_1
      ;[1 0.3329 0.1823 0.5] Start Sequences depending on which type of Searchlight
      (switch Utilities|FlowControl|Switch|SwitchonE_SearchLightVersion (Variables|Default|GetSearchLight%20Version)
        (:NewEnumerator1
          (CallFunction|RotateSpotlight))
        (:NewEnumerator2
          (bind _outactor (Sequencer|Player|CreateLevelSequencePlayer "/Game/Stealth/Sequences/S_TrainRight.S_TrainRight"))
          (bind _output_get (Variables|Default|SetTrainSequence%20Ref _outactor))
          (Sequencer|Player|Play (Variables|/Script/LevelSequence.LevelSequenceActor|GetSequencePlayer _output_get) :!class /Script/MovieScene.MovieSceneSequencePlayer))))))

(fn ConstructionScript)

(fn TraceEnemies
  (bind _spotlight (Variables|Default|GetSpotLight))
  (bind _returnvalue (Transformation|GetWorldLocation _spotlight))
  (if (not (Variables|Default|GetIsPlayerDetected))
    ;[1 0.5164 0.25 0.5] Generates Multi Sphere trace
    (bind _outhits (Collision|MultiSphereTraceForObjects _returnvalue (+ _returnvalue (* (Math|Vector|GetForwardVector _spotlight) (Variables|/Script/Engine.LocalLightComponent|GetAttenuationRadius _spotlight))) (Variables|Default|GetDetectionRadius) (Utilities|Array|MakeArray "ObjectTypeQuery3") false 0 "None"))
    (Variables|Default|SetIsPlayerDetected false)
    ;[1 0.3854 0.579 0.5] Checks if hit result (player) was valid - sends a line trace to player location
    (for _array_element _outhits
      (Variables|Default|SetArray%20Element "")
      (Utilities|IsValid (.HitActor (Collision|BreakHitResult _array_element))
        (:Is%20Valid
          (bind _returnvalue_2 (Actor|GetActorOfClass "/Game/ThirdPerson/Blueprints/BP_ThirdPersonCharacter.BP_ThirdPersonCharacter_C"))
          (Variables|Default|SetPlayer%20Location (Transformation|GetActorLocation _returnvalue_2))
          (bind _outhit (Collision|LineTraceByChannel (Transformation|GetWorldLocation (Variables|Default|GetSpotLight)) (Transformation|GetActorLocation _returnvalue_2) "TraceTypeQuery1" false (Variables|Default|GetActors%20to%20Ignore) "ForDuration"))
          ;[0.6706 0.3438 1 0.5] Checks if theres a blocking wall detected in front of the player - if not the player is detected
          (bind _output_get (Variables|Default|SetIsPlayerDetected (not (Actor|ActorHasTag (.HitActor (Collision|BreakHitResult _outhit)) "Wall"))))
          (if _output_get
            (Development|PrintString "PlayerDetecting" true true "(R=1.000000,G=0.660000,B=1.000000,A=1.000000)")
            (Variables|Default|SetIsPlayerDetected false)
            (CallFunction|PauseSweep)
            (else
              (return))))))))