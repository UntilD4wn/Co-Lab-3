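; BP_AI is an AI pawn that patrols a looping array of waypoints and chases pawns it sees.
; Actor tags decide whether patrol starts at BeginPlay or on the EnemyAppear event, with a short pause between waypoints.
; PawnSensing and the lightspottedplayer event share one chase move, targeting the pawn from the sensing event.
; A retriggerable delay returns it to patrol shortly after the last trigger.
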(event OnSeePawn(PawnSensing)
  (params (Pawn :type Pawn%20Object%20Reference))
  (AI|AIMoveTo self "0, 0, 0" Pawn 5.0 false
    (:then
      (Utilities|FlowControl|RetriggerableDelay 2.0)
      (CallFunction|FollowWaypoint))))

(event Custom|FollowWaypoint
  (AI|AIMoveTo self "0, 0, 0" (Utilities|Array|Get(acopy) (Variables|Default|Getwaypoints) (Variables|Default|Getcurrentwaypoint)) 5.0 false
    (:OnSuccess
      (Math|Integer|IncrementInt (Variables|Default|Getcurrentwaypoint)
        (:%20%20
          (if (>= (Variables|Default|Getcurrentwaypoint) (Utilities|Array|Length (Variables|Default|Getwaypoints)))
            (Variables|Default|Setcurrentwaypoint 0))
          (Utilities|FlowControl|Delay 0.5)
          (CallFunction|FollowWaypoint))))))

(event Custom|EnemyAppear
  (if (Actor|ActorHasTag self "2")
    (CallFunction|FollowWaypoint)))

(event Custom|light%20spotted%20player
  (AI|AIMoveTo self "0, 0, 0" (stale OnSeePawn(PawnSensing) Pawn) 5.0 false
    (:then
      (Utilities|FlowControl|RetriggerableDelay 2.0)
      (CallFunction|FollowWaypoint))))

(event EventBeginPlay
  (if (Actor|ActorHasTag self "1")
    (CallFunction|FollowWaypoint)))

(fn ConstructionScript)